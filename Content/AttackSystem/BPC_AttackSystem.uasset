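; Auto-attack component for the top-down character that fires bolt projectiles at enemies within an attack-range sphere.
; Enter, exit and death events maintain the target array, and looping timers refresh the target and attempt attacks.
; CanFire gates each shot on a living target and a cooldown derived from AttackSpeed.
; FindClosestTarget never updates its minimum distance, so it effectively picks the last qualifying target rather than the closest.
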(event `self.ReceiveBeginPlay`
  ; Setting sphere collider to the attack range variable
  (bind _asbp_top_down_character (cast `/Game/DamageSystem/Player/BP_TopDownCharacter` (`self.GetOwner`)))
  (`SphereComponent.SetSphereRadius` (`/Game/DamageSystem/Player/BP_TopDownCharacter.AttackRangeSphere` _asbp_top_down_character) (`self.AttackRange`) true)
  ; Timer that updates the target every x seconds
  (bind _returnvalue (`KismetSystemLibrary.K2_SetTimerDelegate` (delegate `UpdateTargetSelection`) 0.2 true))
  (set `self.TargetSelectionTimerHandle` _returnvalue)
  ; Attack Check system
  (bind _returnvalue_2 (`KismetSystemLibrary.K2_SetTimerDelegate` (delegate `CheckForAttack`) 0.05 true true))
  (set `self.AttackCheckTimerHandle` _returnvalue_2))

(event `UpdateTargetSelection`
  ; Timer that updates the target every x seconds
  (`self.FindClosestTarget`))

(event `CheckForAttack`
  ; Attack Check system
  (`self.AttemptAttack`))

(event `OnTargetEnteredRange`
  (params (TargetActor :type "/Game/DamageSystem/BPI_Damageable Interface"))
  (bind _targetsinarray (`self.TargetsInArray`))
  ; Adds or removes targets from the array list when they entre, exit the sphere collider
  (`KismetArrayLibrary.Array_AddUnique` _targetsinarray TargetActor)
  (`KismetSystemLibrary.PrintString` "Enemy Added")
  (`self.FindClosestTarget`)
  (if (not (`KismetArrayLibrary.Array_IsEmpty` _targetsinarray))
    (set `self.CanAttack` true)))

(event `ResetAttackCooldown`
  ; Event to reset attack cooldown
  (set `self.CanAttack` true))

(event `OnTargetExitRange`
  (params (TargetActor :type "/Game/DamageSystem/BPI_Damageable Interface"))
  (bind _targetsinarray (`self.TargetsInArray`))
  ; Adds or removes targets from the array list when they entre, exit the sphere collider
  (`KismetArrayLibrary.Array_RemoveItem` _targetsinarray TargetActor)
  (`KismetSystemLibrary.PrintString` "Enemy Removed")
  (`self.FindClosestTarget`)
  (if (`KismetArrayLibrary.Array_IsEmpty` _targetsinarray)
    (set `self.CanAttack` false)))

(event `OnTargetDied`
  (params (DyingTarget :type "/Game/DamageSystem/BPI_Damageable Interface"))
  ; Removes dead targets from the array
  (`KismetArrayLibrary.Array_RemoveItem` (`self.TargetsInArray`) DyingTarget)
  (`self.FindClosestTarget`))

(event `AttemptAttack`
  ; Execute attack logic
  (if (`self.CanFire`)
    (bind _asenemy (cast `/Game/DamageSystem/Enemy/Enemy` (`self.Target`)))
    (`|SpawnActorFromClass` "/Game/Projectiles/BP_Projectile_Bolt.BP_Projectile_Bolt_C" (`SceneComponent.K2_GetComponentToWorld` (`self.ShootPoint`)) "Undefined" "MultiplyWithRoot" (`self.GetOwner`) 500.0 0.0 _asenemy false 3000.0 (`self.MagicDamage`) null)
    (`KismetSystemLibrary.PrintString` "Attacked!")
    (set `self.CanAttack` false)
    (`self.StartAttackCooldown`)))

(fn `CanFire`
  (returns (CanFire :type Boolean))
  (bind _target (`self.Target`))
  (bind _asenemy (cast `/Game/DamageSystem/Enemy/Enemy` _target))
  (return (and (and (`KismetSystemLibrary.IsValidInterface` _target) (`self.CanAttack`)) (not (`/Game/DamageSystem/BPC_DamageSystem.IsDead` (`/Game/DamageSystem/Enemy/Enemy.BPC_DamageSystem` _asenemy))))))

(fn `FindClosestTarget`
  (locals (LocalBestTarget :type "/Game/DamageSystem/BPI_Damageable Interface") (LocalMinDistanceSq :type "Float (double-precision)" :default 99999999.0))
  (set `local.LocalBestTarget` null)
  (bind _output_get (set `local.LocalMinDistanceSq` 99999999.0))
  (for _array_element (`self.TargetsInArray`)
    (bind _location (`/Game/DamageSystem/BPI_Damageable.GetLocation` _array_element))
    (bind _returnvalue (`KismetMathLibrary.Vector_Distance` _location (`Actor.K2_GetActorLocation` (`self.GetOwner`))))
    (if (< (* _returnvalue _returnvalue) _output_get)
      (set `local.LocalBestTarget` _array_element)))
  (set `self.Target` (`local.LocalBestTarget`)))

(fn `StartAttackCooldown`
  (bind _returnvalue (`KismetSystemLibrary.K2_SetTimer` null "ResetAttackCooldown" (/ 1.0 (`self.AttackSpeed`))))
  (set `self.NewVar` _returnvalue))